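; BP_CatheterPort is a catheter port whose spline-mesh tube latches onto a syringe and follows it.
; The construction script builds a spline mesh per segment, keeping only the last in SplineMesh.
; PortArea overlap stores the first ISyringe actor.
; Each Tick moves the final spline point to that syringe's attach point, re-fits the stored mesh (ending on the last segment), and sweeps PortArea to the tip.
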(event OnComponentBeginOverlap(PortArea)
  (params (OverlappedComponent :type Primitive%20Component%20Object%20Reference) (OtherActor :type Actor%20Object%20Reference) (OtherComp :type Primitive%20Component%20Object%20Reference) (OtherBodyIndex :type Integer) (bFromSweep :type Boolean) (SweepResult :type Hit%20Result%20Structure%20%28by%20ref%29))
  (Variables|Default|GetSyringe
    (:then)
    (:else
      (if (Utilities|DoesObjectImplementInterface OtherActor "/Game/Blueprints/Interfaces/ISyringe.ISyringe_C")
        (Variables|Default|SetSyringe OtherActor)))))

(event EventTick
  (params (DeltaSeconds :type Float%20%28single-precision%29))
  (Utilities|FlowControl|Sequence
    (:then_0
      (bind _syringe (Variables|Default|GetSyringe)
        (:then
          (CallFunction|FollowSyringe _syringe))
        (:else)))))

(fn ConstructionScript
  (bind _spline (Variables|Default|GetSpline))
  (for _index (range 0 (- (Spline|GetNumberOfSplinePoints (Variables|Default|GetSpline)) 2))
    (bind _returnvalue (AddComponent|AddSplineMeshComponent false))
    (bind _output_get (Variables|Default|SetSplineMesh _returnvalue))
    (SplineMesh|SetForwardAxis _output_get "X" true)
    (SplineMesh|SetStartandEnd _returnvalue (Spline|GetLocationatSplinePoint _spline _index "Local") (Spline|GetTangentatSplinePoint _spline _index "Local") (Spline|GetLocationatSplinePoint _spline (+ _index 1) "Local") (Spline|GetTangentatSplinePoint _spline (+ _index 1) "Local") true :!class /Script/Engine.SplineMeshComponent)))

(fn FollowSyringe
  (params (Syringe :type Actor%20Object%20Reference))
  (bind _spline (Variables|Default|GetSpline))
  (bind _spline_2 (Variables|Default|GetSpline))
  (bind _spline_3 (Variables|Default|GetSpline))
  (bind _attachworldlocation (Class|ISyringe|GetAttachPoint(Message) Syringe))
  (Spline|SetLocationatSplinePoint _spline_2 (- (Spline|GetNumberOfSplinePoints _spline_2) 1) _attachworldlocation "World" true)
  (for _index (range 0 (- (Spline|GetNumberOfSplinePoints (Variables|Default|GetSpline)) 2))
    (SplineMesh|SetStartandEnd (Variables|Default|GetSplineMesh) (Spline|GetLocationatSplinePoint _spline _index "Local") (Spline|GetTangentatSplinePoint _spline _index "Local") (Spline|GetLocationatSplinePoint _spline (+ _index 1) "Local") (Spline|GetTangentatSplinePoint _spline (+ _index 1) "Local") true :!class /Script/Engine.SplineMeshComponent))
  (Transformation|SetWorldLocation (Variables|Default|GetPortArea) (Spline|GetLocationatSplinePoint _spline_3 (- (Spline|GetNumberOfSplinePoints _spline_3) 1) "World") true false))