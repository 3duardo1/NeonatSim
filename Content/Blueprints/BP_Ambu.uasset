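; BP_Ambu is an Ambu resuscitator bag actor that can appear with or without a mask.
; The construction script calls its parent, then SetState swaps the static mesh according to the NoMask flag.
; An ActionAxis event stores the incoming axis value as Press, with no further use in this file.
; GetAttachPoint exposes the world location of its AttachPoint component.
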(event EventActionAxis
  (params (Axis :type Float%20%28single-precision%29))
  (Variables|Default|SetPress Axis))

(fn ConstructionScript
  (|CallParentFunction)
  (CallFunction|SetState (Variables|Ambu|GetNoMask)))

(fn SetState
  (params (withoutMask :type Boolean))
  (bind _mesh (Variables|Character|GetMesh))
  (if withoutMask
    (Components|StaticMesh|SetStaticMesh _mesh "/Game/Assets/Ambu/Geometries/SM_AmbuNoMask.SM_AmbuNoMask")
    (else
      (Components|StaticMesh|SetStaticMesh _mesh "/Game/Assets/Ambu/Geometries/SM_Ambu_mask90.SM_Ambu_mask90"))))

(fn GetAttachPoint
  (return (Transformation|GetWorldLocation (Variables|Default|GetattachPoint))))