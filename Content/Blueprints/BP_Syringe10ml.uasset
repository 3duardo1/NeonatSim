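; Syringe Blueprint (10 ml) whose plunger and medication material follow an analog action axis input.
; BeginPlay puts a dynamic medication material on the StaticMesh.
; ActionAxis only advances on a new maximum press, so the plunger never retracts; it moves the plunger along local Z, updates the material's "Amount" parameter and prints the value.
; GetAttachPoint returns the AttachPoint's world location; the construction script's plunger logic is unconnected.
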(event EventBeginPlay
  (bind _returnvalue (Rendering|Material|CreateDynamicMaterialInstance "/Game/Assets/Syringe/M_SyringeMed_Inst.M_SyringeMed_Inst" "None" "None" :!class /Script/Engine.KismetMaterialLibrary))
  (bind _output_get (Variables|Default|SetMedMaterial _returnvalue))
  (Rendering|Material|SetMaterial (Variables|Default|GetStaticMesh) 0 _output_get))

(event EventActionAxis
  (params (Axis :type Float%20%28single-precision%29))
  (bind _output_get (Variables|Default|SetPress Axis))
  (if (>= (Variables|Default|GetPress) (Variables|Default|GetPressedAmount))
    (bind _output_get_2 (Variables|Default|SetPressedAmount (Variables|Default|GetPress)))
    (Development|PrintString (Utilities|String|ToString(Float) _output_get_2))
    (Utilities|SetRelativeLocationZ (Variables|Default|GetSM_Jeringa1ML_Plunger) (- (* _output_get 7.0) 7.0) false false)
    (Rendering|Material|SetScalarParameterValue (Variables|Default|GetMedMaterial) "Amount" (Variables|Default|GetPressedAmount) :!class /Script/Engine.MaterialInstanceDynamic)))

(fn ConstructionScript
  (|CallParentFunction))

(fn GetAttachPoint
  (return (Transformation|GetWorldLocation (Variables|Default|GetattachPoint))))