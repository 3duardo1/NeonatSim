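; BP_Catheter is a hand-held catheter item for a VR simulation that detects when it is placed in the trachea.
; Its Sphere overlap with a "trahea"-tagged component reports in-place state through CallInPlace.
; On overlap it caches the holding BP_MotionController_SimHand and opens a Tick-driven gate that fires short haptic pulses.
; Ending the overlap or dropping the item closes the gate, while Action inputs do nothing.
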(event OnComponentBeginOverlap(Sphere)
  (params (OverlappedComponent :type Primitive%20Component%20Object%20Reference) (OtherActor :type Actor%20Object%20Reference) (OtherComp :type Primitive%20Component%20Object%20Reference) (OtherBodyIndex :type Integer) (bFromSweep :type Boolean) (SweepResult :type Hit%20Result%20Structure%20%28by%20ref%29))
  (if (Components|ComponentHasTag OtherComp "trahea")
    (bind _asbp_motion_controller_sim_hand (Utilities|Casting|CastToBP_MotionController_SimHand (Actor|GetAttachParentActor)))
    (Default|CallInPlace true)
    (Utilities|FlowControl|Gate true) ; enters at Open
  ))

(event OnComponentEndOverlap(Sphere)
  (params (OverlappedComponent :type Primitive%20Component%20Object%20Reference) (OtherActor :type Actor%20Object%20Reference) (OtherComp :type Primitive%20Component%20Object%20Reference) (OtherBodyIndex :type Integer))
  (if (Components|ComponentHasTag OtherComp "trahea")
    (Default|CallInPlace false)
    (Utilities|FlowControl|Gate true) ; enters at Close
  ))

(event EventAction)

(event EventTick
  (params (DeltaSeconds :type Float%20%28single-precision%29))
  (Utilities|FlowControl|Gate true
    (:Exit
      (Default|SetHaptics (stale OnComponentBeginOverlap(Sphere) _asbp_motion_controller_sim_hand) (Utilities|Struct|MakeStruct_Haptics_Definition "NewEnumerator3" 0.05 0.15))
      (Default|ExecuteHaptic (stale OnComponentBeginOverlap(Sphere) _asbp_motion_controller_sim_hand) 0.01 0.0 0.0))))

(event EventActionAxis
  (params (Axis :type Float%20%28single-precision%29)))

(event EventDrop
  (|CallParentFunction)
  (Utilities|FlowControl|Gate true) ; enters at Close
)

(fn ConstructionScript
  (|CallParentFunction))