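; BP_TubePath is an actor that animates a short spline mesh segment travelling along a spline path.
; On BeginPlay, if a BP_Newborn exists in the level, it adds a SplineMeshComponent at runtime and attaches it to the root.
; A timeline maps its alpha to distance along the spline, updating the segment's start, end and tangents so the fixed-length piece bends along the curve.
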(event EventBeginPlay
  (bind _spline (Variables|Default|GetSpline))
  (bind _returnvalue (Actor|GetActorOfClass "/Game/Blueprints/BP_Newborn.BP_Newborn_C"))
  (Utilities|IsValid _returnvalue
    (:Is%20Valid
      (bind _returnvalue_2 (AddComponent|AddSplineMeshComponent true))
      (bind _output_get (Variables|Default|SetMeshComponent _returnvalue_2))
      (Transformation|AttachComponentToComponent _output_get (Variables|Default|GetDefaultSceneRoot) "None" "KeepRelative" "KeepRelative" "KeepRelative" true)
      (bind _0_1 (Timeline|Timeline_0 PlayFromStart)
        (:Update
          (Variables|Default|SetSplineLocation (Math|Float|Lerp 0.0 (Spline|GetSplineLength _spline) _0_1))
          (SplineMesh|SetStartandEnd (Variables|Default|GetMeshComponent) (Spline|GetLocationatDistanceAlongSpline _spline (Variables|Default|GetSplineLocation) "Local") (Spline|GetTangentatDistanceAlongSpline _spline (Variables|Default|GetSplineLocation) "Local") (Spline|GetLocationatDistanceAlongSpline _spline (+ (Variables|Default|GetSplineLocation) 15.0) "Local") (Spline|GetTangentatDistanceAlongSpline _spline (+ (Variables|Default|GetSplineLocation) 15.0) "Local") true :!class /Script/Engine.SplineMeshComponent))))))

(fn ConstructionScript)