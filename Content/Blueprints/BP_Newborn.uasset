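; BP_Newborn is an actor whose skeletal mesh alternates between spinning and standing still.
; Tick adds a fixed yaw step each frame, independent of delta time, while Stop is false.
; A looping two-second timer snaps the mesh to the actor rotation saved at BeginPlay and toggles Stop through a FlipFlop.
; Logic building Spline2 from numbered mesh sockets exists but is disconnected and never runs.
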(event Custom|asd
  (Transformation|SetWorldRotation (Variables|SkeletalMeshActor|GetSkeletalMeshComponent) (Variables|Default|GetNewVar_0) true true)
  (Utilities|FlowControl|FlipFlop
    (:A
      (Variables|Default|Setstop true))
    (:B
      (Variables|Default|Setstop false))))

(event EventBeginPlay
  (Utilities|Time|SetTimerbyEvent (delegate Custom|asd) 2.0 true)
  (Variables|Default|SetNewVar_0 (Transformation|GetActorRotation)))

(event Collision|EventActorBeginOverlap
  (params (OtherActor :type Actor%20Object%20Reference)))

(event EventTick
  (params (DeltaSeconds :type Float%20%28single-precision%29))
  (if (not (Variables|Default|Getstop))
    (Transformation|AddWorldRotation (Variables|SkeletalMeshActor|GetSkeletalMeshComponent) "0,1.000000, 0" true true)))

(fn ConstructionScript)