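; BP_Tweezer is a tweezer tool that picks up and releases BP_Catheter actors based on an analog press value.
; When ActionAxis exceeds 0.8, every catheter overlapping HandPoseTrigger is attached to the tweezer, keeping its world transform.
; At lower non-zero values it detaches all attached actors, while a value of zero changes nothing.
; The begin-overlap event is empty, with leftover unconnected class-check and gate nodes.
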(event OnComponentBeginOverlap(HandPoseTrigger)
  (params (OverlappedComponent :type Primitive%20Component%20Object%20Reference) (OtherActor :type Actor%20Object%20Reference) (OtherComp :type Primitive%20Component%20Object%20Reference) (OtherBodyIndex :type Integer) (bFromSweep :type Boolean) (SweepResult :type Hit%20Result%20Structure%20%28by%20ref%29)))

(event EventActionAxis
  (params (Axis :type Float%20%28single-precision%29))
  (bind _output_get (Variables|Default|SetPress Axis))
  (if (> _output_get 0.8)
    (for _array_element (Collision|GetOverlappingActors (Variables|Default|GetHandPoseTrigger) "/Game/Blueprints/BP_Catheter.BP_Catheter_C" :!class /Script/Engine.PrimitiveComponent)
      (Transformation|AttachActorToActor _array_element self "None" "KeepWorld" "KeepWorld" "KeepWorld" true))
    (elif (> _output_get 0.0)
      (for _array_element_2 (Actor|GetAttachedActors true)
        (Utilities|IsValid _array_element_2
          (:Is%20Valid
            (Transformation|DetachFromActor _array_element_2 "KeepWorld" "KeepWorld" "KeepWorld")))))))

(fn ConstructionScript
  (|CallParentFunction))