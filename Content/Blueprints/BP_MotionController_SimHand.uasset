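; VR motion-controller hand for a simulation with newborn and laryngoscopy interactions, driving posed fingers on a skeletal mesh.
; Grab attaches interface-based pickups, eases them into their attachment transform on Tick, and can enable axis-driven finger curl between poses.
; Held objects receive action messages, while InitLaryngoRoutine spawns an instrument directly into the hand.
; Touching "Newborn Sides" switches to a collisionless compress pose, reset by timer after contact ends.
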(event OnComponentBeginOverlap(Capsule)
  (params (OverlappedComponent :type Primitive%20Component%20Object%20Reference) (OtherActor :type Actor%20Object%20Reference) (OtherComp :type Primitive%20Component%20Object%20Reference) (OtherBodyIndex :type Integer) (bFromSweep :type Boolean) (SweepResult :type Hit%20Result%20Structure%20%28by%20ref%29))
  (switch name (Utilities|Array|Get(acopy) (Variables|/Script/Engine.ActorComponent|GetComponentTags OtherComp))
    (:newbornSides
      (Utilities|Time|ClearandInvalidateTimerbyHandle (Variables|Default|Gettimer))
      (Collision|SetCollisionEnabled (Variables|Default|GetHandSkeletalMesh) "NoCollision")
      (Class|HandSkeletalMeshComponent|SetFingersPose (Variables|Default|GetHandSkeletalMesh) "Compress"))))

(event OnComponentEndOverlap(Capsule)
  (params (OverlappedComponent :type Primitive%20Component%20Object%20Reference) (OtherActor :type Actor%20Object%20Reference) (OtherComp :type Primitive%20Component%20Object%20Reference) (OtherBodyIndex :type Integer))
  (switch name (Utilities|Array|Get(acopy) (Variables|/Script/Engine.ActorComponent|GetComponentTags OtherComp))
    (:newbornSides
      (bind _returnvalue (Utilities|Time|SetTimerbyEvent (delegate Custom|ResetFingers) 2.0))
      (Variables|Default|Settimer _returnvalue))))

(event OnComponentEndOverlap(GrabTrigger)
  (params (OverlappedComponent :type Primitive%20Component%20Object%20Reference) (OtherActor :type Actor%20Object%20Reference) (OtherComp :type Primitive%20Component%20Object%20Reference) (OtherBodyIndex :type Integer)))

(event Custom|ResetFingers
  (Collision|SetCollisionEnabled (Variables|Default|GetHandSkeletalMesh) "QueryAndPhysics")
  (Class|HandSkeletalMeshComponent|SetFingersPose (Variables|Default|GetHandSkeletalMesh) "idle"))

(event EventBeginPlay
  (|CallParentFunction)
  (Class|HandSkeletalMeshComponent|SetFingersPose (Variables|Default|GetHandSkeletalMesh) "idle"))

(event Collision|EventActorBeginOverlap
  (params (OtherActor :type Actor%20Object%20Reference))
  (|CallParentFunction OtherActor) ; This node is disabled and will not be called.\nDrag off pins to build functionality.
)

(event EventTick
  (params (DeltaSeconds :type Float%20%28single-precision%29))
  (|CallParentFunction DeltaSeconds)
  (if (Variables|Default|GetisGrabbing)
    (CallFunction|InterpolateActortoHand DeltaSeconds)))

(event Custom|InitLaryngoRoutine
  (params (pose :type Name) (InstrumentalClass :type Actor%20Class%20Reference))
  (Class|HandSkeletalMeshComponent|SetFingersPose (Variables|Default|GetHandSkeletalMesh) pose)
  (if (Utilities|IsValidClass InstrumentalClass)
    (bind _returnvalue (Game|SpawnActorfromClass InstrumentalClass (Math|Transform|MakeTransform "0, 0, 0" "0, 0, 0" "1,1,1") "Undefined" self 0))
    (bind _objectinfo (Class|IObjectInteractive|GetObjectInfo(Message) _returnvalue))
    (Transformation|AttachComponentToComponent _returnvalue (Variables|Default|GetHandSkeletalMesh) "None" "KeepWorld" "KeepWorld" "KeepWorld" true)
    (Transformation|SetActorRelativeTransform _returnvalue (.attachmenttransform _objectinfo) false false)
    (Variables|Default|SetObjectInHand _returnvalue)))

(fn ConstructionScript
  (|CallParentFunction)
  (Class|HandSkeletalMeshComponent|BuildRig (Variables|Default|GetHandSkeletalMesh)))

(fn Grab
  (bind _handskeletalmesh (Variables|Default|GetHandSkeletalMesh))
  (bind _array_element (Utilities|Array|ForEachLoopwithBreak (Collision|GetOverlappingActors (Variables|Default|GetGrabTrigger) "/Script/Engine.Actor" :!class /Script/Engine.PrimitiveComponent) :!label _label)
    (:LoopBody
      (if (Utilities|DoesObjectImplementInterface _array_element "/Game/Blueprints/Interfaces/IObjectInteractive.IObjectInteractive_C")
        (bind _objectinfo (Class|IObjectInteractive|GetObjectInfo(Message) _array_element))
        (if (.canpickup _objectinfo)
          (Variables|Default|SetObjectInHand _array_element)
          (Variables|Default|SetisGrabbing true)
          (Variables|Default|SetObjRelativeTransform (.attachmenttransform _objectinfo))
          (Class|IObjectInteractive|PickUp(Message) _array_element)
          (Class|HandSkeletalMeshComponent|SetFingersPose _handskeletalmesh (.getgrabposename _objectinfo))
          (Transformation|AttachComponentToComponent _array_element _handskeletalmesh "None" "KeepWorld" "KeepWorld" "KeepWorld" true)
          (CallFunction|SetHaptics (Utilities|Struct|MakeStruct_Haptics_Definition "NewEnumerator3" 0.08 0.2))
          (CallFunction|ExecuteHaptic 0.01 0.0 0.0)
          (goto _label Break))
        (elif (Utilities|DoesObjectImplementInterface _array_element "/Game/Blueprints/Interfaces/IObjectManipulative.IObjectManipulative_C")
          (Development|PrintString "CLOTH FOUND" true true "(R=1.000000,G=0.000000,B=0.853144,A=1.000000)")
          (Class|IObjectManipulative|Grab(Message) _array_element))))))

(fn Drop
  (bind _handskeletalmesh (Variables|Default|GetHandSkeletalMesh))
  (bind _objectinhand (Variables|Default|GetObjectInHand)
    (:then
      (Transformation|DetachFromActor _objectinhand "KeepWorld" "KeepWorld" "KeepWorld")
      (Class|IObjectInteractive|Drop(Message) _objectinhand)
      (Class|HandSkeletalMeshComponent|SetFingersPose _handskeletalmesh "idle")
      (Class|HandSkeletalMeshComponent|ApplyVRInput _handskeletalmesh 0.0 0.0 0.0 0.0 0.0)
      (Variables|Default|SetObjectInHand 0))
    (:else)))

(fn InterpolateActortoHand
  (params (Delta :type Float%20%28single-precision%29))
  (bind _objrelativetransform (Variables|Default|GetObjRelativeTransform))
  (bind _handskeletalmesh (Variables|Default|GetHandSkeletalMesh))
  (bind _objectinhand (Variables|Default|GetObjectInHand)
    (:then
      (bind _output_get (LocalVariables|SetbIsFinished (< (Math|Vector|VectorLengthSquared (- (.location (Class|KismetMathLibrary|TInterpto (Transformation|GetRelativeTransform (Variables|/Script/Engine.Actor|GetRootComponent _objectinhand)) (Variables|Default|GetObjRelativeTransform) Delta 1e+01)) (.location _objrelativetransform))) 0.2)))
      (if _output_get
        (LocalVariables|SetNewTransform (Variables|Default|GetObjRelativeTransform))
        (else
          (LocalVariables|SetNewTransform (Math|Transform|MakeTransform (.location (Class|KismetMathLibrary|TInterpto (Transformation|GetRelativeTransform (Variables|/Script/Engine.Actor|GetRootComponent _objectinhand)) (Variables|Default|GetObjRelativeTransform) Delta 1e+01)) (.rotation (Class|KismetMathLibrary|TInterpto (Transformation|GetRelativeTransform (Variables|/Script/Engine.Actor|GetRootComponent _objectinhand)) (Variables|Default|GetObjRelativeTransform) Delta 1e+01)) (.scale _objrelativetransform)))))
      (Transformation|SetActorRelativeTransform (Variables|Default|GetObjectInHand) (LocalVariables|GetNewTransform) false false)
      (Variables|Default|SetisGrabbing (not (LocalVariables|GetbIsFinished)))
      (if (LocalVariables|GetbIsFinished)
        (bind _objectinfo (Class|IObjectInteractive|GetObjectInfo(Message) (Variables|Default|GetObjectInHand)))
        (if (Utilities|Name|NotEqual(Name) (.endinterpolationname _objectinfo) "None")
          (Class|HandSkeletalMeshComponent|SetVRInputReferencePose _handskeletalmesh (.getgrabposename _objectinfo))
          (Class|HandSkeletalMeshComponent|SetVRInputGripPose _handskeletalmesh (.endinterpolationname _objectinfo))
          (return))
        (else
          (return))))
    (:else)))

(fn ActionAxis
  (params (Axis :type Float%20%28single-precision%29))
  (if (> Axis 0.0)
    (bind _objectinhand (Variables|Default|GetObjectInHand)
      (:then
        (Class|IObjectInteractive|ActionAxis(Message) _objectinhand Axis)
        (bind _objectinfo (Class|IObjectInteractive|GetObjectInfo(Message) (Variables|Default|GetObjectInHand)))
        (if (Utilities|Name|NotEqual(Name) (.endinterpolationname _objectinfo) "None")
          (Class|HandSkeletalMeshComponent|ApplyVRInput (Variables|Default|GetHandSkeletalMesh) Axis Axis Axis Axis Axis)))
      (:else))))

(fn AxisHaptic
  (params (Axis :type Float%20%28single-precision%29))
  (if (> Axis 0.0)
    (CallFunction|SetHaptics (Utilities|Struct|MakeStruct_Haptics_Definition "NewEnumerator3" 0.05 0.15))
    (CallFunction|ExecuteHaptic 0.01 0.0 0.0)
    (else
      (Utilities|FlowControl|DoOnce false) ; enters at Reset
    )))

(fn Action
  (Class|IObjectInteractive|Action(Message) (Variables|Default|GetObjectInHand)))