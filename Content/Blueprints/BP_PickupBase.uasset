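; Base pickup actor for objects that can be picked up, dropped and sent back to their starting transform.
; PickUp and Drop flip the first flag in ObjectInfo, which carries attachment and grab pose data, and toggle mesh physics when PhysicsOnRelease is set.
; ReturntoStart disables physics and teleports the actor to the transform cached at BeginPlay.
; GetObjectInfo exposes the struct, while GetAttachmentMesh is an empty stub.
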(event EventReturntoStart
  (Physics|SetSimulatePhysics (Variables|Default|GetMesh) false)
  (Transformation|SetActorTransform (Variables|Default|GetstartLocation) false true))

(event EventBeginPlay
  (Variables|Default|SetstartLocation (Transformation|GetActorTransform)))

(event EventPickUp
  (Variables|Default|SetObjectInfo (Utilities|Struct|MakeS_ObjectInteractiveInfo false (.attachmenttransform (Variables|Default|GetObjectInfo)) (.getgrabposename (Variables|Default|GetObjectInfo)) (.endinterpolationname (Variables|Default|GetObjectInfo))))
  (if (Variables|General|GetphysicsOnRelease)
    (Physics|SetSimulatePhysics (Variables|Default|GetMesh) false)))

(event EventDrop
  (Variables|Default|SetObjectInfo (Utilities|Struct|MakeS_ObjectInteractiveInfo true (.attachmenttransform (Variables|Default|GetObjectInfo)) (.getgrabposename (Variables|Default|GetObjectInfo)) (.endinterpolationname (Variables|Default|GetObjectInfo))))
  (if (Variables|General|GetphysicsOnRelease)
    (Physics|SetSimulatePhysics (Variables|Default|GetMesh) true)))

(fn ConstructionScript)

(fn GetAttachmentMesh
  (return 0))

(fn GetObjectInfo
  (return (Variables|Default|GetObjectInfo)))