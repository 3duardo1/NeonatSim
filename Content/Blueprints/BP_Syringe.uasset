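; BP_Syringe is a syringe whose plunger and medication level follow an analog press axis.
; On BeginPlay it creates a dynamic instance of the medication material on its mesh.
; The axis event keeps the highest press reached in NewVar0, so the plunger cannot retract.
; That value sets the plunger's relative Z and the material's "Amount" parameter, and is printed to screen.
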(event EventBeginPlay
  (bind _returnvalue (Rendering|Material|CreateDynamicMaterialInstance (Variables|Default|GetStaticMesh) 0 "/Game/Assets/Syringe/M_SyringeMed_Inst.M_SyringeMed_Inst" "None" :!class /Script/Engine.PrimitiveComponent))
  (Variables|Default|SetMedMaterial _returnvalue))

(event EventTick
  (params (DeltaSeconds :type Float%20%28single-precision%29)))

(event EventActionAxis
  (params (Axis :type Float%20%28single-precision%29))
  (bind _output_get (Variables|Default|SetPress Axis))
  (if (>= (Variables|Default|GetPress) (Variables|Default|GetNewVar_0))
    (bind _output_get_2 (Variables|Default|SetNewVar_0 (Variables|Default|GetPress)))
    (Development|PrintString (Utilities|String|ToString(Float) _output_get_2))
    (Utilities|SetRelativeLocationZ (Variables|Default|GetSM_Jeringa1ML_Plunger) (- (* _output_get 6.0) 6.0) false false)
    (Rendering|Material|SetScalarParameterValue (Variables|Default|GetMedMaterial) "Amount" (- (* _output_get 6.0) 6.0) :!class /Script/Engine.MaterialInstanceDynamic)))

(fn ConstructionScript
  (|CallParentFunction))