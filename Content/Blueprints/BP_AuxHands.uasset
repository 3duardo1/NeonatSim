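; BP_AuxHands is an auxiliary hand actor that automatically loops an Ambu bag squeeze animation.
; On BeginPlay it initializes a body solver with camera, motion controllers and hand mesh, then sets Ambu rest and pressed poses.
; A timeline feeds simulated VR finger-curl input, updates Press and nudges the hand in world space.
; Compress replays the timeline in bursts of three, pauses, then calls itself again indefinitely.
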(event Custom|Compress
  (bind (_direction _alpha _hand_movement) (Timeline|PressureTime PlayFromStart)
    (:Update
      (Variables|Default|SetPress _alpha)
      (Class|HandSkeletalMeshComponent|ApplyVRInput (Variables|Default|GetHandSkeletalMesh) _alpha _alpha _alpha _alpha _alpha)
      (Transformation|AddWorldOffset (Variables|Default|GetHandSkeletalMesh) (Math|Vector|MakeVector (* _hand_movement 0.035) 0.0 (* _hand_movement 0.035)) false false))
    (:Finished
      (Math|Integer|IncrementInt (Variables|Default|GettimesCompressed)
        (:%20%20
          (if (< (Variables|Default|GettimesCompressed) 3)
            (Timeline|PressureTime PlayFromStart)
            (else
              (Variables|Default|SettimesCompressed 0)
              (Utilities|FlowControl|Delay 1.0)
              (CallFunction|Compress))))))))

(event EventBeginPlay
  (bind _handskeletalmesh (Variables|Default|GetHandSkeletalMesh))
  (Class|BodySolverComponent|Initialize (Variables|Default|GetBodySolver) (Variables|Default|GetCamera) (Variables|Default|GetMotionControllerR) (Variables|Default|GetMotionControllerL) (Variables|Default|GetHandSkeletalMesh))
  (Class|HandSkeletalMeshComponent|SetFingersPose _handskeletalmesh "Ambu")
  (Class|HandSkeletalMeshComponent|SetVRInputReferencePose _handskeletalmesh "Ambu")
  (Class|HandSkeletalMeshComponent|SetVRInputGripPose _handskeletalmesh "AmbuPressed")
  (CallFunction|Compress))

(fn ConstructionScript
  (Class|HandSkeletalMeshComponent|BuildRig (Variables|Default|GetHandSkeletalMesh)))