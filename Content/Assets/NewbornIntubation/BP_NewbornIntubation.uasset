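; Newborn intubation Blueprint whose tongue mesh can be moved by a laryngoscope and springs back when released.
; When BP_Laryngoscope overlaps the tongue, the tongue attaches to the touching component and any return animation stops.
; Moving too far from its starting transform, or any end overlap on the delay-enabled Box, detaches it and plays a timeline lerping it home.
; The tongue's own end overlap only prints debug text, and leftover height-constraint logic is disconnected.
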(event OnComponentBeginOverlap(SM_Tongue_Intu)
  (params (OverlappedComponent :type Primitive%20Component%20Object%20Reference) (OtherActor :type Actor%20Object%20Reference) (OtherComp :type Primitive%20Component%20Object%20Reference) (OtherBodyIndex :type Integer) (bFromSweep :type Boolean) (SweepResult :type Hit%20Result%20Structure%20%28by%20ref%29))
  (bind _tongueinittransform (Variables|Default|GetTongueInitTransform))
  (bind _sm_tongue_intu (Variables|Default|GetSM_Tongue_Intu))
  (bind _sm_tongue_intu_2 (Variables|Default|GetSM_Tongue_Intu))
  (if (== (Utilities|GetClass OtherActor) "/Game/Blueprints/BP_Laryngoscope.BP_Laryngoscope_C")
    (Development|PrintString "LARINGO IN" true true "(R=0.211112,G=1.000000,B=0.000000,A=1.000000)")
    (Transformation|AttachComponentToComponent _sm_tongue_intu OtherComp "None" "KeepWorld" "KeepWorld" "KeepWorld" true)
    (Transformation|SetWorldScale3D _sm_tongue_intu (.scale (Variables|Default|GetTongueInitTransform)))
    (Variables|Default|SetTongueAttached true)
    (bind _alpha (Timeline|Timeline_0 Stop)
      (:Update
        (Transformation|SetWorldTransform _sm_tongue_intu_2 (Math|Transform|MakeTransform (Math|Vector|Lerp(Vector) (Transformation|GetWorldLocation _sm_tongue_intu_2) (.location _tongueinittransform) _alpha) (Math|Rotator|Lerp(Rotator) (Transformation|GetWorldRotation _sm_tongue_intu_2) (.rotation _tongueinittransform) _alpha) (.scale (Variables|Default|GetTongueInitTransform))) false false)))))

(event OnComponentEndOverlap(SM_Tongue_Intu)
  (params (OverlappedComponent :type Primitive%20Component%20Object%20Reference) (OtherActor :type Actor%20Object%20Reference) (OtherComp :type Primitive%20Component%20Object%20Reference) (OtherBodyIndex :type Integer))
  ;[1 1 1] Utter bullshit
  (if (== (Utilities|GetClass OtherActor) "/Game/Blueprints/BP_Laryngoscope.BP_Laryngoscope_C")
    (Development|PrintString "LARINGO OUT" true true "(R=0.972238,G=0.000000,B=1.000000,A=1.000000)")
    (Utilities|FlowControl|Sequence)))

(event OnComponentEndOverlap(Box)
  (params (OverlappedComponent :type Primitive%20Component%20Object%20Reference) (OtherActor :type Actor%20Object%20Reference) (OtherComp :type Primitive%20Component%20Object%20Reference) (OtherBodyIndex :type Integer))
  (bind _tongueinittransform (Variables|Default|GetTongueInitTransform))
  (bind _sm_tongue_intu (Variables|Default|GetSM_Tongue_Intu))
  (Transformation|DetachFromComponent (Variables|Default|GetSM_Tongue_Intu) "KeepWorld" "KeepWorld" "KeepWorld" true)
  (Transformation|SetWorldScale3D (Variables|Default|GetSM_Tongue_Intu) (.scale (Variables|Default|GetTongueInitTransform)))
  (bind _alpha (Timeline|Timeline_0 PlayFromStart)
    (:Update
      (Transformation|SetWorldTransform _sm_tongue_intu (Math|Transform|MakeTransform (Math|Vector|Lerp(Vector) (Transformation|GetWorldLocation _sm_tongue_intu) (.location _tongueinittransform) _alpha) (Math|Rotator|Lerp(Rotator) (Transformation|GetWorldRotation _sm_tongue_intu) (.rotation _tongueinittransform) _alpha) (.scale (Variables|Default|GetTongueInitTransform))) false false))))

(event EventBeginPlay
  (Variables|Default|SetTongueInitTransform (Transformation|GetWorldTransform (Variables|Default|GetSM_Tongue_Intu)))
  (Utilities|FlowControl|Delay 1.0)
  (Collision|SetCollisionEnabled (Variables|Default|GetBox) "QueryOnly"))

(event EventTick
  (params (DeltaSeconds :type Float%20%28single-precision%29))
  (bind _tongueinittransform (Variables|Default|GetTongueInitTransform))
  (bind _sm_tongue_intu (Variables|Default|GetSM_Tongue_Intu))
  (if (Variables|Default|GetTongueAttached)
    (if (> (Math|Vector|Distance(Vector) (.location (Variables|Default|GetTongueInitTransform)) (Transformation|GetWorldLocation (Variables|Default|GetSM_Tongue_Intu))) 2e+01)
      (Variables|Default|SetTongueAttached false)
      (Transformation|DetachFromComponent (Variables|Default|GetSM_Tongue_Intu) "KeepWorld" "KeepWorld" "KeepWorld" true)
      (Transformation|SetWorldScale3D (Variables|Default|GetSM_Tongue_Intu) (.scale (Variables|Default|GetTongueInitTransform)))
      (bind _alpha (Timeline|Timeline_0 PlayFromStart)
        (:Update
          (Transformation|SetWorldTransform _sm_tongue_intu (Math|Transform|MakeTransform (Math|Vector|Lerp(Vector) (Transformation|GetWorldLocation _sm_tongue_intu) (.location _tongueinittransform) _alpha) (Math|Rotator|Lerp(Rotator) (Transformation|GetWorldRotation _sm_tongue_intu) (.rotation _tongueinittransform) _alpha) (.scale (Variables|Default|GetTongueInitTransform))) false false))))))

(fn ConstructionScript)