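; Manager Blueprint that keeps a registry of teleport locations and switches them on or off as a group.
; Functions add locations uniquely, remove them or return the list.
; Activate and deactivate calls loop over the list, setting each valid location's state.
; If either loop meets an invalid reference, it then rebuilds the array with only the valid, unique entries.
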(event EventBeginPlay)

(event Collision|EventActorBeginOverlap
  (params (OtherActor :type Actor%20Object%20Reference)))

(event EventTick
  (params (DeltaSeconds :type Float%20%28single-precision%29)))

(fn ConstructionScript)

(fn GetTeleportLocations
  (return (Variables|Default|GetTeleportLocations)))

(fn ActivateTeleportLocations
  (for _array_element (Variables|Default|GetTeleportLocations)
    (Utilities|IsValid _array_element
      (:Is%20Valid
        (Default|ActivateTeleportLocation _array_element true))
      (:Is%20Not%20Valid
        (LocalVariables|SetCheckArray true))))
  (if (LocalVariables|GetCheckArray)
    (CallFunction|CheckTeleportLocationArray)))

(fn DeactivateTeleportLocations
  (for _array_element (Variables|Default|GetTeleportLocations)
    (Utilities|IsValid _array_element
      (:Is%20Valid
        (Default|ActivateTeleportLocation _array_element false))
      (:Is%20Not%20Valid
        (LocalVariables|SetCheckArray true))))
  (if (LocalVariables|GetCheckArray)
    (CallFunction|CheckTeleportLocationArray)))

(fn AddTeleportLocation
  (params (TeleportLocation :type Comp%20Teleport%20Object%20Reference))
  (Utilities|Array|AddUnique (Variables|Default|GetTeleportLocations) TeleportLocation))

(fn RemoveTeleportLocation
  (params (TeleportLocation :type Comp%20Teleport%20Object%20Reference))
  (Utilities|Array|RemoveItem (Variables|Default|GetTeleportLocations) TeleportLocation))

(fn CheckTeleportLocationArray
  (for _array_element (Variables|Default|GetTeleportLocations)
    (Utilities|IsValid _array_element
      (:Is%20Valid
        (Utilities|Array|AddUnique (LocalVariables|GetTemporaryArray) _array_element))))
  (Variables|Default|SetTeleportLocations (LocalVariables|GetTemporaryArray)))