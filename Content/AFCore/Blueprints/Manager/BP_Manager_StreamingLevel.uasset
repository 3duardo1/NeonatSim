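; Manager that swaps streamed environment levels from an indexed list, loading the current index on BeginPlay.
; Each switch fades the player camera out, unloads the old level, loads the new one, fades back in and broadcasts the change.
; Levels flagged AR stop or start the mobile pawn's AR session.
; Next and Prev both call the same wrapping increment, with no visible difference in direction.
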(event Custom|LoadStreamLevel
  (params (Index :type Integer) (Force :type Boolean) (Pawn :type BP%20Pawn%20Base%20Object%20Reference) (FadeDuration :type Float%20%28single-precision%29))
  (if (or Force (!= Index (Variables|Default|GetCurrentlyLoadedIndex)))
    (Utilities|Fade FadeDuration "Forward" Pawn)
    (Utilities|FlowControl|Sequence
      (:then_0
        (if (.ar (Variables|Default|GetCurrentlyLoadedLevel))
          (bind _asbp_pawn_mobile (Utilities|Casting|CastToBP_Pawn_Mobile Pawn)
            (:then
              (Default|StopARSession _asbp_pawn_mobile))
            (:CastFailed
              _)))
        (Utilities|IsValid (Class|GameplayStatics|GetStreamingLevel (.levelname (Variables|Default|GetCurrentlyLoadedLevel)))
          (:Is%20Valid
            (if (Class|LevelStreaming|IsLevelLoaded (Class|GameplayStatics|GetStreamingLevel (.levelname (Variables|Default|GetCurrentlyLoadedLevel))))
              (Game|UnloadStreamLevel(byName) (.levelname (Variables|Default|GetCurrentlyLoadedLevel)) false)))))
      (:then_1
        (bind _output_get (Variables|Default|SetCurrentlyLoadedLevel (Utilities|Array|Get(acopy) (Variables|Default|GetAvailableStreamLevels) Index)))
        (Game|LoadStreamLevel(byName) (.levelname _output_get) true)
        (Variables|Default|SetCurrentlyLoadedIndex Index)
        (Utilities|Fade FadeDuration "Backward" Pawn)
        (Default|CallNewStreamLevelLoaded (Variables|Default|GetCurrentlyLoadedIndex) (CallFunction|GetEnviromentInfo))
        (if (.ar (Variables|Default|GetCurrentlyLoadedLevel))
          (bind _asbp_pawn_mobile_2 (Utilities|Casting|CastToBP_Pawn_Mobile Pawn))
          (EventDispatchers|AssignAROriginFound _asbp_pawn_mobile_2 (delegate Custom|AROriginFound_Event_0))
          (Default|InitiateARSession _asbp_pawn_mobile_2))))))

(event Custom|AROriginFound_Event_0
  (params (Pawn :type BP%20Pawn%20Mobile%20Object%20Reference))
  (EventDispatchers|UnbindEventfromAROriginFound Pawn (delegate Custom|AROriginFound_Event_0))
  (Development|PrintString "AROrigin"))

(event Custom|SetNextEnviroment
  (params (Pawn :type BP%20Pawn%20Base%20Object%20Reference) (FadeDuration :type Float%20%28single-precision%29))
  (CallFunction|LoadStreamLevel (CallFunction|IncrementIntwithModulo (Variables|Default|GetCurrentlyLoadedIndex) (Utilities|Array|Length (Variables|Default|GetAvailableStreamLevels))) false Pawn FadeDuration))

(event Custom|SetPrevEnviroment
  (params (Pawn :type BP%20Pawn%20Base%20Object%20Reference) (FadeDuration :type Float%20%28single-precision%29))
  (CallFunction|LoadStreamLevel (CallFunction|IncrementIntwithModulo (Variables|Default|GetCurrentlyLoadedIndex) (Utilities|Array|Length (Variables|Default|GetAvailableStreamLevels))) false Pawn FadeDuration))

(event EventBeginPlay
  (CallFunction|LoadStreamLevel (Variables|Default|GetCurrentlyLoadedIndex) true 0 0.5))

(fn ConstructionScript)

(fn GetEnviromentInfo
  (return (Utilities|Array|Get(acopy) (Variables|Default|GetAvailableStreamLevels) (Variables|Default|GetCurrentlyLoadedIndex))))