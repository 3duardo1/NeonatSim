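; VR simulation pawn that drives two sim hands and a body solver.
; Once controllers are ready, it casts them to left and right hands and initializes the solver with camera, controllers and hand meshes.
; Grips grab and drop, also notifying the first test cloth actor on press; triggers drive hand actions and haptics.
; A laryngoscopy event only scales both controllers, leaving its pose and instrument setup unconnected.
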(event Custom|StartHandSetup
  (CallFunction|GetSimHands)
  (Class|BodySolverComponent|Initialize (Variables|Default|GetBodySolver) (Variables|Default|GetMainCamera) (Variables|Default|GetMotionControllerRight) (Variables|Default|GetMotionControllerLeft) (Variables|/Game/AFCore/Blueprints/VR/MotionControllers/BP_MotionController_SimHand.BP_MotionController_SimHand_C|GetHandSkeletalMesh (Variables|Default|GetRightHand)) (Variables|/Game/AFCore/Blueprints/VR/MotionControllers/BP_MotionController_SimHand.BP_MotionController_SimHand_C|GetHandSkeletalMesh (Variables|Default|GetLeftHand)))
  (Development|PrintString "Hello"))

(event EventBeginPlay
  (|CallParentFunction)
  (EventDispatchers|BindEventtoControllersReady (delegate Custom|StartHandSetup))
  (bind _outactors (Actor|GetAllActorsOfClass "/Game/VICOD/BP_TestCloth.BP_TestCloth_C"))
  (Variables|Default|SetCloth (Utilities|Array|Get(acopy) _outactors)))

(event EventTick
  (params (DeltaSeconds :type Float%20%28single-precision%29))
  (|CallParentFunction DeltaSeconds))

(event Input|ActionEvents|InputActionMotionControllerTriggerLeft
  (params (Key :type Key%20Structure))
  (:Pressed
    (Default|Action (Variables|Default|GetLeftHand))))

(event Input|ActionEvents|InputActionMotionControllerGripLeft
  (params (Key :type Key%20Structure))
  (bind _lefthand (Variables|Default|GetLeftHand))
  (:Pressed
    (Default|Grab _lefthand)
    (bind _outactors (Actor|GetAllActorsOfClass "/Game/VICOD/BP_TestCloth.BP_TestCloth_C"))
    (bind _output_get (Variables|Default|SetCloth (Utilities|Array|Get(acopy) _outactors)))
    (Class|IObjectManipulative|Grab(Message) _output_get))
  (:Released
    (Default|Drop _lefthand)))

(event Input|ActionEvents|InputActionMotionControllerGripRight
  (params (Key :type Key%20Structure))
  (bind _righthand (Variables|Default|GetRightHand))
  (:Pressed
    (Default|Grab _righthand)
    (bind _outactors (Actor|GetAllActorsOfClass "/Game/VICOD/BP_TestCloth.BP_TestCloth_C"))
    (bind _output_get (Variables|Default|SetCloth (Utilities|Array|Get(acopy) _outactors)))
    (Class|IObjectManipulative|Grab(Message) _output_get))
  (:Released
    (Default|Drop _righthand)))

(event Input|ActionEvents|InputActionMotionControllerTriggerRight
  (params (Key :type Key%20Structure))
  (:Pressed
    (Default|Action (Variables|Default|GetRightHand))))

(event Input|AxisEvents|InputAxisTriggerAxisRight
  (params (AxisValue :type Float%20%28single-precision%29))
  (bind _righthand (Variables|Default|GetRightHand))
  (Default|ActionAxis _righthand AxisValue)
  (if (> AxisValue 0.1)
    (Default|SetHaptics _righthand (Utilities|Struct|MakeStruct_Haptics_Definition "NewEnumerator3" 0.1 AxisValue))
    (Default|ExecuteHaptic _righthand 0.01 0.0 0.0)))

(event Input|AxisEvents|InputAxisTriggerAxisLeft
  (params (AxisValue :type Float%20%28single-precision%29))
  (bind _lefthand (Variables|Default|GetLeftHand))
  (Default|ActionAxis _lefthand AxisValue)
  (if (> AxisValue 0.1)
    (Default|SetHaptics _lefthand (Utilities|Struct|MakeStruct_Haptics_Definition "NewEnumerator3" 0.1 AxisValue))
    (Default|ExecuteHaptic _lefthand 0.01 0.0 0.0)))

(event Custom|InitLaryngoRoutine
  (Transformation|SetWorldScale3D (Variables|Default|GetMotionControllerLeft) "10.000000,10.000000,10.000000")
  (Transformation|SetWorldScale3D (Variables|Default|GetMotionControllerRight) "10.000000,10.000000,10.000000"))

(fn ConstructionScript
  (|CallParentFunction))

(fn GetSimHands
  (bind _asbp_motion_controller_sim_hand_left (Utilities|Casting|CastToBP_MotionController_SimHand_Left (Variables|Default|GetLeftController))
    (:then
      (Variables|Default|SetLeftHand _asbp_motion_controller_sim_hand_left)
      (bind _asbp_motion_controller_sim_hand_right (Utilities|Casting|CastToBP_MotionController_SimHand_Right (Variables|Default|GetRightController))
        (:then
          (Variables|Default|SetRightHand _asbp_motion_controller_sim_hand_right)
          (return))
        (:CastFailed
          _)))
    (:CastFailed
      _))
  (Development|PrintString "Controllers are misconfigurated. Check Comp_Controlls/MotionControllerSet"))