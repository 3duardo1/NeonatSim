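; BP_Helper_Ping is a short-lived ping effect actor that plays a sound at its location and shows an animated sphere pulse.
; Its construction script gives the inner and outer spheres a shared dynamic M_Ping material with configurable thickness and color.
; On BeginPlay, a timeline scales only the outer sphere by the Size variable and animates material opacity, then the actor destroys itself.
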(event EventBeginPlay
  (Audio|PlaySoundatLocation (Variables|Default|GetSound) (Transformation|GetActorLocation) "0, 0, 0" 1.0 1.0 0.0 0 0 0)
  (bind (_direction _scale _opacity) (Timeline|PingAnimation PlayFromStart)
    (:Update
      (Transformation|SetWorldScale3D (Variables|Default|GetOuterSphere) (Math|Conversions|ToVector(Float) (* _scale (Variables|Default|GetSize))))
      (Rendering|Material|SetScalarParameterValue (Variables|Default|GetMaterial) "AnimatedOpacity" _opacity :!class /Script/Engine.MaterialInstanceDynamic))
    (:Finished
      (Actor|DestroyActor))))

(fn ConstructionScript
  (bind _returnvalue (Rendering|Material|CreateDynamicMaterialInstance "/Game/AFCore/Materials/Ping/M_Ping.M_Ping" "None" "None" :!class /Script/Engine.KismetMaterialLibrary))
  (bind _output_get (Variables|Default|SetMaterial _returnvalue))
  (Rendering|Material|SetMaterial (Variables|Default|GetOuterSphere) 0 _output_get)
  (Rendering|Material|SetScalarParameterValue (Variables|Default|GetMaterial) "Thickness" (Variables|Default|GetThickness) :!class /Script/Engine.MaterialInstanceDynamic)
  (Rendering|Material|SetVectorParameterValue (Variables|Default|GetMaterial) "Color" (Variables|Default|GetColor) :!class /Script/Engine.MaterialInstanceDynamic))