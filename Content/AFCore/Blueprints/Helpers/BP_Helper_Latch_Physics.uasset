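; BP_Helper_Latch_Physics is a latch helper actor that joins a handle to an attached component through a physics constraint.
; On BeginPlay it constrains Handle to the attached component at the given socket.
; If the constraint breaks, it sends the grabbing-actor release message to the latching actor.
; When destroyed, it breaks the constraint and then unbinds the break event.
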(event Custom|OnConstraintBroken_Event_0
  (params (ConstraintIndex :type Integer))
  (Class|InterfaceGrabbingActor|GrabbingActorReleaseActor(Message) (Variables|Default|GetLatchingActor)))

(event Custom|OnDestroyed_Event_0
  (params (DestroyedActor :type Actor%20Object%20Reference))
  (Class|PhysicsConstraintComponent|BreakConstraint (Variables|Default|GetPhysicsConstraint))
  (EventDispatchers|UnbindEventfromOnConstraintBroken (Variables|Default|GetPhysicsConstraint) (delegate Custom|OnConstraintBroken_Event_0)))

(event EventBeginPlay
  (|CallParentFunction)
  (Class|PhysicsConstraintComponent|SetConstrainedComponents (Variables|Default|GetPhysicsConstraint) (Variables|Default|GetHandle) "None" (.AsPrimitive%20Component (Utilities|Casting|CastToPrimitiveComponent (Variables|Default|GetAttachedComponent))) (Variables|Default|GetAttachedSocket))
  (EventDispatchers|AssignOnConstraintBroken (Variables|Default|GetPhysicsConstraint) (delegate Custom|OnConstraintBroken_Event_0))
  (Game|AssignOnDestroyed (delegate Custom|OnDestroyed_Event_0)))

(fn ConstructionScript
  (|CallParentFunction))

(fn Get
  (return 0))