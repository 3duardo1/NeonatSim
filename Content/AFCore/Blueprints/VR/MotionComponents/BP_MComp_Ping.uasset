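; VR motion component that lets a player place a ping marker in the world when the Ping function input is set.
; It traces a short line on the Visibility channel forward from the select/search arrow, taking the hit location or the trace end if nothing is hit.
; The VR pawn spawns the ping at that point, tinted with the player state's index color.
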(event EventFunctionInput
  (params (Function :type Name :default "None") (Set :type Boolean))
  (bind _vrpawn (Variables|Default|GetVRPawn))
  ;[1 1 1] KeyInputs
  (|CallParentFunction Function Set)
  (switch name Function
    (:Ping
      ;[1 1 1] Ping
      (if Set
        (bind _impactpoint (|TraceForPing))
        (Default|SpawnPing _vrpawn "0, 0, 0" _impactpoint 2.0 8.0 (Default|GetIndexColor (Default|GetPlayerState _vrpawn)))))))

(fn ConstructionScript)