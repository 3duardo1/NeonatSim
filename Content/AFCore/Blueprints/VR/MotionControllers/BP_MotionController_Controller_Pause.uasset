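; VR motion controller Blueprint variant that keeps working while the game is paused.
; On BeginPlay it runs the parent logic, marks itself tickable when paused, then calls SetupControllerMesh.
; Despite its name, SetupControllerMesh here only loops over the actor's Timeline components and makes each tickable during pause.
; Tick and the construction script just defer to the parent class.
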(event EventBeginPlay
  ;[1 1 1] Setup
  (|CallParentFunction)
  (Class|Actor|SetTickablewhenPaused true)
  (|SetupControllerMesh))

(event EventTick
  (params (DeltaSeconds :type Float%20%28single-precision%29))
  (|CallParentFunction DeltaSeconds))

(fn ConstructionScript
  (|CallParentFunction))